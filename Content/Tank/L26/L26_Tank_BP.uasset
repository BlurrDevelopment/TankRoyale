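; L26 player tank pawn Blueprint that wires player input to tank driving, aiming, firing, camera control and pickups.
; BeginPlay hands the barrel, turret and tracks to TankAiming and TankMovement components, which handle firing, gadgets, launch speed and movement intents.
; Tick polls GameModeDeathmatch so driving, firing and gadgets wait for match start.
; A gimbal and pitch-clamped spring arm provide look, zoom and first/third-person swapping; per-track throttle inputs are left unconnected.
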(event EventTick
  (params (DeltaSeconds :type Float%20%28single-precision%29))
  (bind _asgame_mode_deathmatch (Utilities|Casting|CastToGameModeDeathmatch (Game|GetGameMode)))
  (bind _returnvalue (Class|GameModeDeathmatch|HasGameStarted _asgame_mode_deathmatch))
  (Variables|Default|SetGameStarted _returnvalue))

(event Collision|EventActorBeginOverlap
  (params (OtherActor :type Actor%20Object%20Reference)))

(event EventBeginPlay
  (Class|TankAimingComponent|Initialise (Variables|Default|GetTankAiming) self (Variables|Default|GetBarrel) (Variables|Default|GetTurret))
  (Class|TankMovementComponent|Initialise (Variables|Default|GetTankMovement) (Variables|Default|GetLeft%20Track) (Variables|Default|GetRightTrack)))

(event Input|ActionEvents|InputActionFire
  (params (Key :type Key%20Structure))
  ;[1 1 1] Firing
  (:Pressed
    (if (Variables|Default|GetGameStarted)
      (Class|TankAimingComponent|Fire (Variables|Default|GetTankAiming)))))

(event Input|ActionEvents|InputActionIncreaseLaunchSpeed
  (params (Key :type Key%20Structure))
  ;[1 1 1] Launch Speed Adjustment
  (:Pressed
    (Class|TankAimingComponent|IncreaseLaunchSpeed (Variables|Default|GetTankAiming))))

(event Input|ActionEvents|InputActionDecreaseLaunchSpeed
  (params (Key :type Key%20Structure))
  ;[1 1 1] Launch Speed Adjustment
  (:Pressed
    (Class|TankAimingComponent|DecreaseLaunchSpeed (Variables|Default|GetTankAiming))))

(event Input|ActionEvents|InputActionUseGadget
  (params (Key :type Key%20Structure))
  ;[1 1 1] Fire Gadget
  (:Pressed
    (if (Variables|Default|GetGameStarted)
      (Class|TankAimingComponent|FireGadget (Variables|Default|GetTankAiming)))))

(event Input|ActionEvents|InputActionSwapCam
  (params (Key :type Key%20Structure))
  ;[1 1 1] Switch Camera
  (:Pressed
    (Components|Activation|ToggleActive (Variables|Default|Get3rd%20person))
    (Components|Activation|ToggleActive (Variables|Default|Get1st%20person))))

(event Input|AxisEvents|InputAxisTurnRight
  (params (AxisValue :type Float%20%28single-precision%29))
  ;[1 1 1] Turn Right
  (if (Variables|Default|GetGameStarted)
    (Class|TankMovementComponent|IntendTurnRight (Variables|Default|GetTankMovement) AxisValue)))

(event Input|AxisEvents|InputAxisCameraZoom
  (params (AxisValue :type Float%20%28single-precision%29))
  (bind _springarm (Variables|Default|GetSpringArm))
  ;[1 1 1] Camera Zoom
  (Variables|/Script/Engine.SpringArmComponent|SetTargetArmLength _springarm (Math|Float|Clamp(Float) (+ AxisValue (Variables|/Script/Engine.SpringArmComponent|GetTargetArmLength _springarm)) (Variables|Default|GetMinimum%20Camera%20Zoom) (Variables|Default|GetMaximum%20Camera%20Zoom))))

(event Input|AxisEvents|InputAxisLeftTrackThrottle
  (params (AxisValue :type Float%20%28single-precision%29))
  ;[1 1 1] Throttle Left
  (if (Variables|Default|GetGameStarted)
    _))

(event Input|AxisEvents|InputAxisRightTrackThrottle
  (params (AxisValue :type Float%20%28single-precision%29))
  ;[1 1 1] Throttle Right
  (if (Variables|Default|GetGameStarted)
    _))

(event Input|AxisEvents|InputAxisAimAzimuth
  (params (AxisValue :type Float%20%28single-precision%29))
  ;[1 1 1] X Axis Aim
  (Transformation|AddLocalRotation (Variables|Default|GetAzimuth%20Gimbal) (Math|Rotator|MakeRotator 0.0 0.0 (* AxisValue (Utilities|Time|GetWorldDeltaSeconds) 85.0)) false false))

(event Input|AxisEvents|InputAxisAimElevation
  (params (AxisValue :type Float%20%28single-precision%29))
  (bind _springarm (Variables|Default|GetSpringArm))
  ;[1 1 1] Y Axis Aim  26/10
  (Transformation|AddLocalRotation _springarm (Math|Rotator|MakeRotator 0.0 (* AxisValue (Utilities|Time|GetWorldDeltaSeconds) 85.0) 0.0) false false)
  (CallFunction|ClampCameraPitchAngle (.pitch (Transformation|GetWorldRotation _springarm)) _springarm))

(event Input|AxisEvents|InputAxisMoveForward
  (params (AxisValue :type Float%20%28single-precision%29))
  ;[1 1 1] Move Forward
  (if (Variables|Default|GetGameStarted)
    (Class|TankMovementComponent|IntendMoveForward (Variables|Default|GetTankMovement) AxisValue)))

(event Input|ActionEvents|InputActionPickup
  (params (Key :type Key%20Structure))
  (:Released
    (if (Variables|Default|GetbOnPickup)
      (Class|Tank|UsePickup))))

(fn ConstructionScript)

(fn ClampCameraPitchAngle
  (params (CurrentPitch :type Float%20%28single-precision%29) (SpringArm :type Scene%20Component%20Object%20Reference))
  (bind _maximum_camera_angle (Variables|Default|GetMaximum%20Camera%20Angle))
  (bind _minimum_camera_angle (Variables|Default|GetMinimum%20Camera%20Angle))
  (if (> CurrentPitch _maximum_camera_angle)
    (Transformation|AddLocalRotation SpringArm (Math|Rotator|MakeRotator 0.0 (- _maximum_camera_angle CurrentPitch) 0.0) false false))
  (if (< CurrentPitch _minimum_camera_angle)
    (Transformation|AddLocalRotation SpringArm (Math|Rotator|MakeRotator 0.0 (- _minimum_camera_angle CurrentPitch) 0.0) false false)))