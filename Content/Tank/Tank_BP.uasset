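; Tank pawn Blueprint for the deathmatch mode, wiring player input, aiming, movement, camera and health bar.
; BeginPlay initialises the TankAiming and TankMovement components, links the health bar widget and registers with the game mode for a team, reporting death to it later.
; Input drives movement intents, gimbal and pitch-clamped spring arm aiming, and first/third-person camera toggling.
; Firing calls TankAiming, with shot sound chosen by firing state and a delayed reload sound.
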(event Custom|OnDeathEvent
  (bind _astank_royale_game_mode_deathmatch_bp (Utilities|Casting|CastToTankRoyaleGameModeDeathmatch_BP (Game|GetGameMode)))
  (Default|TankDeath _astank_royale_game_mode_deathmatch_bp self))

(event EventBeginPlay
  (Class|TankAimingComponent|Initialise (Variables|Default|GetTankAiming) (Variables|Default|GetBarrel) (Variables|Default|GetTurret))
  (Class|TankMovementComponent|Initialise (Variables|Default|GetTankMovement) (Variables|Default|GetLeft%20Track) (Variables|Default|GetRightTrack))
  (CallFunction|InitialiseHealthBarWidget)
  (EventDispatchers|AssignOnDeath (delegate Custom|OnDeathEvent))
  (bind _astank_royale_game_mode_deathmatch_bp (Utilities|Casting|CastToTankRoyaleGameModeDeathmatch_BP (Game|GetGameMode)))
  (Default|AssignTeam _astank_royale_game_mode_deathmatch_bp self))

(event Collision|EventActorBeginOverlap
  (params (OtherActor :type Actor%20Object%20Reference)))

(event EventTick
  (params (DeltaSeconds :type Float%20%28single-precision%29)))

(event Input|ActionEvents|InputActionFire
  (params (Key :type Key%20Structure))
  (bind _tankaiming (Variables|Default|GetTankAiming))
  (bind _barrel (Variables|Default|GetBarrel))
  (bind _returnvalue (Transformation|GetSocketLocation _barrel "Projectile"))
  ;[1 1 1] Firing
  (:Pressed
    (Class|TankAimingComponent|Fire _tankaiming)
    (Audio|PlaySoundatLocation (Utilities|Select :Index (Variables|/Script/TankRoyale.TankAimingComponent|GetFiringState _tankaiming) :Reloading 0 :Aiming "/Game/Audio/Explosion02.Explosion02" :Locked "/Game/Audio/Explosion02.Explosion02" :OutOfAmmo 0) _returnvalue)
    (Utilities|FlowControl|Delay 3.0)
    (Audio|PlaySoundatLocation "/Game/Sounds/418882__kierankeegan__tank-reload.418882__kierankeegan__tank-reload" _returnvalue)))

(event Input|ActionEvents|InputActionSwapCam
  (params (Key :type Key%20Structure))
  ;[1 1 1] Switch Camera
  (:Pressed
    (Components|Activation|ToggleActive (Variables|Default|Get3rd%20person))
    (Components|Activation|ToggleActive (Variables|Default|Get1st%20person))))

(event Input|AxisEvents|InputAxisTurnRight
  (params (AxisValue :type Float%20%28single-precision%29))
  ;[1 1 1] Turn Right
  (Class|TankMovementComponent|IntendTurnRight (Variables|Default|GetTankMovement) AxisValue))

(event Input|AxisEvents|InputAxisLeftTrackThrottle
  (params (AxisValue :type Float%20%28single-precision%29))
  ;[1 1 1] Throttle Left
)

(event Input|AxisEvents|InputAxisRightTrackThrottle
  (params (AxisValue :type Float%20%28single-precision%29))
  ;[1 1 1] Throttle Right
)

(event Input|AxisEvents|InputAxisAimAzimuth
  (params (AxisValue :type Float%20%28single-precision%29))
  ;[1 1 1] X Axis Aim
  (Transformation|AddLocalRotation (Variables|Default|GetAzimuth%20Gimbal) (Math|Rotator|MakeRotator 0.0 0.0 (* AxisValue (Utilities|Time|GetWorldDeltaSeconds) 85.0)) false false))

(event Input|AxisEvents|InputAxisAimElevation
  (params (AxisValue :type Float%20%28single-precision%29))
  (bind _springarm (Variables|Default|GetSpringArm))
  ;[1 1 1] Y Axis Aim  26/10
  (Transformation|AddLocalRotation _springarm (Math|Rotator|MakeRotator 0.0 (* AxisValue (Utilities|Time|GetWorldDeltaSeconds) 85.0) 0.0) false false)
  (CallFunction|ClampCameraPitchAngle (.pitch (Transformation|GetWorldRotation _springarm)) _springarm))

(event Input|AxisEvents|InputAxisMoveForward
  (params (AxisValue :type Float%20%28single-precision%29))
  ;[1 1 1] Move Forward
  (Class|TankMovementComponent|IntendMoveForward (Variables|Default|GetTankMovement) AxisValue))

(fn ConstructionScript)

(fn InitialiseHealthBarWidget
  (bind _ashealth_bar_bp (Utilities|Casting|CastToHealthBar_BP (UserInterface|GetUserWidgetObject (Variables|Default|GetHealth%20Bar))))
  (Variables|/Game/UI/HealthBar_BP.HealthBar_BP_C|SetMyTank _ashealth_bar_bp self))

(fn ClampCameraPitchAngle
  (params (CurrentPitch :type Float%20%28single-precision%29) (SpringArm :type Scene%20Component%20Object%20Reference))
  (bind _maximum_camera_angle (Variables|Default|GetMaximum%20Camera%20Angle))
  (bind _minimum_camera_angle (Variables|Default|GetMinimum%20Camera%20Angle))
  (if (> CurrentPitch _maximum_camera_angle)
    (Transformation|AddLocalRotation SpringArm (Math|Rotator|MakeRotator 0.0 (- _maximum_camera_angle CurrentPitch) 0.0) false false))
  (if (< CurrentPitch _minimum_camera_angle)
    (Transformation|AddLocalRotation SpringArm (Math|Rotator|MakeRotator 0.0 (- _minimum_camera_angle CurrentPitch) 0.0) false false)))