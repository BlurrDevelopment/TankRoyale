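; Deathmatch game mode Blueprint that manages the match's start, in-game and end-game UI.
; On BeginPlay it shows the start widget, waits briefly, then adds the deathmatch UI, stores it as GamemodeUI and calls StartGame.
; Separate events display the end-game screen and forward killer, state and victim to the stored UI's kill feed.
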(event EventBeginPlay
  (bind _returnvalue (UserInterface|CreateWidget "/Game/UI/HUD/GameStart_BP.GameStart_BP_C"))
  (UserInterface|Viewport|AddtoViewport _returnvalue 1)
  (Utilities|FlowControl|Delay 3.0)
  (bind _returnvalue_2 (UserInterface|CreateWidget "/Game/UI/HUD/DeathmatchUI_BP.DeathmatchUI_BP_C"))
  (UserInterface|Viewport|AddtoViewport _returnvalue_2 0)
  (Variables|Default|SetGamemodeUI _returnvalue_2)
  (Class|GameModeDeathmatch|StartGame))

(event EventDisplayEndGameUI
  (bind _returnvalue (UserInterface|CreateWidget "/Game/UI/Menus/EndGame_BP.EndGame_BP_C"))
  (UserInterface|Viewport|AddtoViewport _returnvalue 0))

(event EventAddKilltoFeed
  (params (Killer :type String) (State :type String) (Victim :type String))
  (Default|AddKill (Variables|Default|GetGamemodeUI) Killer State Victim))

(fn ConstructionScript)