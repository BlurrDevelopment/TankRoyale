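; Deathmatch game state Blueprint that drives match UI for the end screen and kill feed.
; DisplayEndGameUI_ creates the EndGame_BP widget and adds it to the viewport.
; AddKillToFeed_1 passes killer, state and victim to GamemodeUI's AddKill.
; The start-screen and delayed DeathmatchUI_BP setup, the only assignment of GamemodeUI here, is unconnected and never runs, as is the StartGame call.
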(event Custom|DisplayEndGameUI_
  (bind _returnvalue (UserInterface|CreateWidget "/Game/UI/Menus/EndGame_BP.EndGame_BP_C"))
  (UserInterface|Viewport|AddtoViewport _returnvalue 0))

(event Custom|AddKillToFeed_1
  (params (Killer :type String) (State :type String) (Victim :type String))
  (Default|AddKill (Variables|Default|GetGamemodeUI) Killer State Victim))

(event EventBeginPlay)

(event EventTick
  (params (DeltaSeconds :type Float%20%28single-precision%29)))

(fn ConstructionScript)