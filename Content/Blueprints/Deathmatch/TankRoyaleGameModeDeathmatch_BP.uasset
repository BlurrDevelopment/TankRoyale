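; Deathmatch game mode Blueprint for Tank Royale that tracks kills and deaths for two teams.
; Kill and death events increment per-team counters, which reset on BeginPlay.
; Every Tick, GetWinningTeam scores each team as kills minus deaths and sets WinningTeam to 1, 2, or 0 for a tie.
; A debug print marks the mode as pending a move to C++.
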(event Custom|TeamTwoKill
  ;[1 1 1] Team Two
  (Variables|Default|SetTeam%20Two%20Kills (+ 1 (Variables|Default|GetTeam%20Two%20Kills))))

(event Custom|TeamTwoDeath
  ;[1 1 1] Team Two
  (Variables|Default|SetTeam%20Two%20Deaths (+ (Variables|Default|GetTeam%20Two%20Deaths) 1)))

(event Custom|TeamOneDeath
  ;[1 1 1] Team One
  (Variables|Default|SetTeam%20One%20Deaths (+ (Variables|Default|GetTeam%20One%20Deaths) 1)))

(event Custom|TeamOneKill
  ;[1 1 1] Team One
  (Variables|Default|SetTeam%20One%20Kills (+ (Variables|Default|GetTeam%20One%20Kills) 1)))

(event EventBeginPlay
  ;[1 1 1] Begin Play
  (Variables|Default|SetTeam%20One%20Kills 0)
  (Variables|Default|SetTeam%20One%20Deaths 0)
  (Variables|Default|SetTeam%20Two%20Kills 0)
  (Variables|Default|SetTeam%20Two%20Deaths 0)
  (Variables|Default|SetTeam%20One%20Score 0)
  (Variables|Default|SetTeam%20Two%20Score 0)
  (Development|PrintString "TODO: Move Deathmatch Gamemode to CPP"))

(event EventTick
  (params (DeltaSeconds :type Float%20%28single-precision%29))
  ;[1 1 1] Tick
  (CallFunction|GetWinningTeam))

(fn ConstructionScript)

(fn GetWinningTeam
  (Variables|Default|SetTeam%20One%20Score (- (Variables|Default|GetTeam%20One%20Kills) (Variables|Default|GetTeam%20One%20Deaths)))
  (Variables|Default|SetTeam%20Two%20Score (- (Variables|Default|GetTeam%20Two%20Kills) (Variables|Default|GetTeam%20Two%20Deaths)))
  (if (> (Variables|Default|GetTeam%20One%20Score) (Variables|Default|GetTeam%20Two%20Score))
    (Variables|Default|SetWinning%20Team 1)
    (elif (> (Variables|Default|GetTeam%20Two%20Score) (Variables|Default|GetTeam%20One%20Score))
      (Variables|Default|SetWinning%20Team 2)
      (else
        (Variables|Default|SetWinning%20Team 0)))))